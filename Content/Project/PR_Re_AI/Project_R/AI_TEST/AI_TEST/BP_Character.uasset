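; BP_Character is an AI test character whose only logic is a sensing check that toggles on a Blackboard player reference.
; CheckPlayerActor tests whether PlayerActorKey holds a valid object, then prints a Korean "someone left" message if so, or "someone entered" if not.
; Both branches write the key with no object value connected, so SensedActor is never stored.
; The event graph and construction script are empty.
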(event EventBeginPlay)

(event Collision|EventActorBeginOverlap
  (params (OtherActor :type Actor%20Object%20Reference)))

(event EventTick
  (params (DeltaSeconds :type Float%20%28single-precision%29)))

(fn ConstructionScript)

(fn CheckPlayerActor
  (params (SensedActor :type Actor%20Object%20Reference))
  (Utilities|IsValid (AI|Components|Blackboard|GetValueasObject (AI|GetBlackboard 0) (Utilities|Name|MakeLiteralName "PlayerActorKey"))
    (:Is%20Valid
      (Development|PrintText "누군가 나갔어")
      (AI|Components|Blackboard|SetValueasObject (AI|GetBlackboard 0) (Utilities|Name|MakeLiteralName "PlayerActorKey") 0))
    (:Is%20Not%20Valid
      (Development|PrintText "누군가 들어왔어")
      (AI|Components|Blackboard|SetValueasObject (AI|GetBlackboard 0) (Utilities|Name|MakeLiteralName "PlayerActorKey") 0))))